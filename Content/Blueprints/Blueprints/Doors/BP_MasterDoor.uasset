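; BP_MasterDoor is a purchasable door in the ZM game mode that costs player points and activates new zones when opened.
; Its trigger shows the player a cost hint on the HUD and caches whether they can afford it.
; Using it wakes net dormancy, rechecks and deducts points, then activates its zone and destroys it.
; A named DoorGroup makes one purchase do this for every door in that group.
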(event OnComponentBeginOverlap(DoorTrigger)
  (params (OverlappedComponent :type Primitive%20Component%20Object%20Reference) (OtherActor :type Actor%20Object%20Reference) (OtherComp :type Primitive%20Component%20Object%20Reference) (OtherBodyIndex :type Integer) (bFromSweep :type Boolean) (SweepResult :type Hit%20Result%20Structure%20%28by%20ref%29))
  (bind _asbp_zmplayer_character (Utilities|Casting|CastToBP_ZMPlayerCharacter OtherActor))
  (Variables|/ZombieSurvival/Core/BP_ZMPlayerCharacter.BP_ZMPlayerCharacter_C|SetShowHintstrings? _asbp_zmplayer_character true)
  (bind _asbp_zmplayer_controller (Utilities|Casting|CastToBP_ZMPlayerController (Pawn|GetController _asbp_zmplayer_character)))
  (if (>= (Variables|/ZombieSurvival/Core/BP_ZMPlayerController.BP_ZMPlayerController_C|GetPoints _asbp_zmplayer_controller) (Variables|Default|GetCost))
    (Variables|Default|SetCanAfford? true)
    (else
      (Variables|Default|SetCanAfford? false)))
  (Utilities|IsValid (Variables|/ZombieSurvival/Core/BP_ZMPlayerController.BP_ZMPlayerController_C|GetHUDWidgetReference _asbp_zmplayer_controller)
    (:Is%20Valid
      (Default|SetHintstring (Variables|/ZombieSurvival/Core/BP_ZMPlayerController.BP_ZMPlayerController_C|GetHUDWidgetReference _asbp_zmplayer_controller) (Utilities|Text|ToText(String) (Utilities|String|Append (Utilities|String|ToString(Text) (Variables|Default|GetHintstring)) (Utilities|String|ToString(Integer) (Variables|Default|GetCost)) " Points"))))))

(event OnComponentEndOverlap(DoorTrigger)
  (params (OverlappedComponent :type Primitive%20Component%20Object%20Reference) (OtherActor :type Actor%20Object%20Reference) (OtherComp :type Primitive%20Component%20Object%20Reference) (OtherBodyIndex :type Integer))
  (bind _asbp_zmplayer_character (Utilities|Casting|CastToBP_ZMPlayerCharacter OtherActor))
  (Variables|/ZombieSurvival/Core/BP_ZMPlayerCharacter.BP_ZMPlayerCharacter_C|SetShowHintstrings? _asbp_zmplayer_character false)
  (bind _asbp_zmplayer_controller (Utilities|Casting|CastToBP_ZMPlayerController (Pawn|GetController _asbp_zmplayer_character)))
  (Utilities|IsValid (Variables|/ZombieSurvival/Core/BP_ZMPlayerController.BP_ZMPlayerController_C|GetHUDWidgetReference _asbp_zmplayer_controller)
    (:Is%20Valid
      (Default|SetHintstring (Variables|/ZombieSurvival/Core/BP_ZMPlayerController.BP_ZMPlayerController_C|GetHUDWidgetReference _asbp_zmplayer_controller)))))

(event Custom|OpenDoor
  (params (PersonWhoOpenedDoor :type BP%20ZM%20Player%20Character%20Object%20Reference))
  (bind _doorgroup (Variables|Default|GetDoorGroup))
  (bind _output_get (Variables|Default|SetPersonWhoOpenedDoor PersonWhoOpenedDoor))
  (bind _asbp_zmplayer_controller (Utilities|Casting|CastToBP_ZMPlayerController (Pawn|GetController _output_get)))
  (if (>= (Variables|/ZombieSurvival/Core/BP_ZMPlayerController.BP_ZMPlayerController_C|GetPoints _asbp_zmplayer_controller) (Variables|Default|GetCost)) ; Do You Have Enough Points?
    (Default|RemovePoints _asbp_zmplayer_controller (Variables|Default|GetCost))
    (bind _asbp_zmgame_mode (Utilities|Casting|CastToBP_ZMGameMode (Game|GetGameMode)))
    (if (Math|Boolean|NORBoolean (Utilities|Name|Equal(Name) _doorgroup "") (Utilities|Name|Equal(Name) _doorgroup "None"))
      ;[1 1 1] Destroy all doors from group
      (bind _outactors (Actor|GetAllActorsOfClass "BP_MasterDoor_C"))
      (for _array_element _outactors
        (if (Utilities|Name|Equal(Name) (Variables|BP_MasterDoor_C|GetDoorGroup _array_element) (Variables|Default|GetDoorGroup))
          (Default|ActivateNewZones _asbp_zmgame_mode (Variables|BP_MasterDoor_C|GetEnteredZoneToActivate _array_element))
          (Actor|DestroyActor _array_element)))
      (else
        (Default|ActivateNewZones _asbp_zmgame_mode (Variables|Default|GetEnteredZoneToActivate))
        (Actor|DestroyActor)))))

(event EventUsed
  (params (Invoker :type Actor%20Object%20Reference))
  (bind _asbp_zmplayer_character (Utilities|Casting|CastToBP_ZMPlayerCharacter Invoker))
  (if (Variables|Default|GetCanAfford?)
    (Networking|SetNetDormancy "DORM_Never")
    (CallFunction|OpenDoor _asbp_zmplayer_character)
    (Variables|Default|SetCanAfford? false)))

(fn ConstructionScript)