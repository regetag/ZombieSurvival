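; Perk machine for a zombies mode that shows a priced hint and hides a one-time point bonus for players who are prone.
; Trigger overlap toggles the character's hint flag and sets or clears the HUD hintstring, built from the hint text and cost.
; The prone bonus is checked only on entering the trigger, then disabled for that machine.
; An affordability helper compares controller points to cost, but no purchase logic exists here.
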(event OnComponentBeginOverlap(MachineTrigger)
  (params (OverlappedComponent :type Primitive%20Component%20Object%20Reference) (OtherActor :type Actor%20Object%20Reference) (OtherComp :type Primitive%20Component%20Object%20Reference) (OtherBodyIndex :type Integer) (bFromSweep :type Boolean) (SweepResult :type Hit%20Result%20Structure%20%28by%20ref%29))
  (bind _asbp_zmplayer_character (Utilities|Casting|CastToBP_ZMPlayerCharacter OtherActor))
  (Variables|/ZombieSurvival/Core/BP_ZMPlayerCharacter.BP_ZMPlayerCharacter_C|SetShowHintstrings? _asbp_zmplayer_character true)
  (CallFunction|HandleProneReward _asbp_zmplayer_character)
  (bind _asbp_zmplayer_controller (Utilities|Casting|CastToBP_ZMPlayerController (Pawn|GetController _asbp_zmplayer_character)))
  (Utilities|IsValid (Variables|/ZombieSurvival/Core/BP_ZMPlayerController.BP_ZMPlayerController_C|GetHUDWidgetReference _asbp_zmplayer_controller)
    (:Is%20Valid
      (bind _hintstring (CallFunction|MakeHintString))
      (Default|SetHintstring (Variables|/ZombieSurvival/Core/BP_ZMPlayerController.BP_ZMPlayerController_C|GetHUDWidgetReference _asbp_zmplayer_controller) _hintstring))))

(event OnComponentEndOverlap(MachineTrigger)
  (params (OverlappedComponent :type Primitive%20Component%20Object%20Reference) (OtherActor :type Actor%20Object%20Reference) (OtherComp :type Primitive%20Component%20Object%20Reference) (OtherBodyIndex :type Integer))
  (bind _asbp_zmplayer_character (Utilities|Casting|CastToBP_ZMPlayerCharacter OtherActor))
  (Variables|/ZombieSurvival/Core/BP_ZMPlayerCharacter.BP_ZMPlayerCharacter_C|SetShowHintstrings? _asbp_zmplayer_character false)
  (bind _asbp_zmplayer_controller (Utilities|Casting|CastToBP_ZMPlayerController (Pawn|GetController _asbp_zmplayer_character)))
  (Utilities|IsValid (Variables|/ZombieSurvival/Core/BP_ZMPlayerController.BP_ZMPlayerController_C|GetHUDWidgetReference _asbp_zmplayer_controller)
    (:Is%20Valid
      (Default|SetHintstring (Variables|/ZombieSurvival/Core/BP_ZMPlayerController.BP_ZMPlayerController_C|GetHUDWidgetReference _asbp_zmplayer_controller)))))

(fn ConstructionScript)

(fn HandleProneReward
  (params (ZMPlayerCharacter :type BP%20ZM%20Player%20Character%20Object%20Reference))
  (if (and (Variables|Default|GetProneRewardAvailable) (Variables|/Script/DonkehFramework.DFBaseCharacter|GetbIsProne ZMPlayerCharacter))
    (Variables|Default|SetProneRewardAvailable false)
    (bind _asbp_zmplayer_controller (Utilities|Casting|CastToBP_ZMPlayerController (Pawn|GetController ZMPlayerCharacter)))
    (Default|AddPoints _asbp_zmplayer_controller (Variables|Default|GetProneRewardAmount))))

(fn MakeHintString
  (return (Utilities|Text|ToText(String) (Utilities|String|Append (Utilities|String|ToString(Text) (Variables|Default|GetHintstring)) (Utilities|String|ToString(Integer) (Variables|Default|GetCost)) " Points"))))

(fn DoPlayerCanAfford
  (params (ZMPlayerCharacter :type BP%20ZM%20Player%20Character%20Object%20Reference))
  (bind _asbp_zmplayer_controller (Utilities|Casting|CastToBP_ZMPlayerController (Pawn|GetController ZMPlayerCharacter)))
  (return (>= (Variables|/ZombieSurvival/Core/BP_ZMPlayerController.BP_ZMPlayerController_C|GetPoints _asbp_zmplayer_controller) (Variables|Default|GetCost))))